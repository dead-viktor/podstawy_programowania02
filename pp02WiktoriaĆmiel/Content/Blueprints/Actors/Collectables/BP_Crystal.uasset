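; BP_Crystal is a collectable crystal that vanishes into the player's pawn (the ball) on overlap, then destroys itself.
; Overlap caches the pawn's location and the crystal's scale, location and light intensity, then plays the TL_BlendAlpha timeline.
; Timeline tracks drive lerps that shrink the crystal, dim its point light and move it to the cached ball location.
; The move lerps from world origin, leaving the cached crystal location unused.
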(event EventBeginPlay)

(event EventTick
  (params (DeltaSeconds :type Float%20%28single-precision%29)))

(event Collision|EventActorBeginOverlap
  (params (OtherActor :type Actor%20Object%20Reference))
  (Utilities|IsPlayer OtherActor (Game|Player|GetPlayerPawn 0)
    (:IsPlayer
      (CallFunction|SetVariables)
      (bind (_direction _crystallocation _crystalscale _crystallight) (Timeline|TL_BlendAlpha Play)
        (:Update
          (CallFunction|MoveCrystal "0, 0, 0" _crystallocation)
          (CallFunction|ResizeCrystal _crystalscale)
          (CallFunction|DimLightCrystal _crystallight))
        (:Finished
          (Actor|DestroyActor))))))

(fn ConstructionScript)

(fn MoveCrystal
  (params (A :type Vector) (Alpha :type Float%20%28single-precision%29))
  (Transformation|SetActorLocation (Math|Vector|Lerp(Vector) A (Variables|Default|GetBallLocation) Alpha) false false))

(fn ResizeCrystal
  (params (Alpha :type Float%20%28single-precision%29))
  (Transformation|SetActorScale3D (Math|Vector|Lerp(Vector) (Variables|Default|GetCrystalScale) "0, 0, 0" Alpha)))

(fn DimLightCrystal
  (params (Alpha :type Float%20%28single-precision%29))
  (Rendering|Components|Light|SetIntensity (Variables|Default|GetPointLight) (Math|Float|Lerp (Variables|Default|GetCrystalLight) 0.0 Alpha)))

(fn SetVariables
  (Variables|Default|SetCrystalScale (Transformation|GetActorScale3D))
  (Variables|Default|SetCrystalLight (Variables|/Script/Engine.LightComponentBase|GetIntensity (Variables|Default|GetPointLight)))
  (Variables|Default|SetBallLocation (Transformation|GetActorLocation (Game|Player|GetPlayerPawn 0)))
  (Variables|Default|SetCrystalLocation (Transformation|GetActorLocation)))