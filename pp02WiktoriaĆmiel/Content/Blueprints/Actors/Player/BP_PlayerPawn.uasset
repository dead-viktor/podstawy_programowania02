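; Player pawn for a rolling ball that restarts the level when it takes any damage.
; Both movement input axes feed one function that applies horsepower-scaled acceleration torque to the ball.
; The camera fades in from black on BeginPlay; damage triggers a macro that fades to red, waits out the fade, then reopens the current level.
; AdjustCamera sets spring arm length and rotations but is not called within this Blueprint.
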(event EventBeginPlay
  (CallFunction|TurnCameraon))

(event Collision|EventActorBeginOverlap
  (params (OtherActor :type Actor%20Object%20Reference)))

(event EventTick
  (params (DeltaSeconds :type Float%20%28single-precision%29)))

(event Game|Damage|EventAnyDamage
  (params (Damage :type Float%20%28single-precision%29) (DamageType :type Damage%20Type%20Object%20Reference) (InstigatedBy :type Controller%20Object%20Reference) (DamageCauser :type Actor%20Object%20Reference))
  (Utilities|RestartLevel))

(event Input|AxisEvents|InputAxisfowards-backwards
  (params (AxisValue :type Float%20%28single-precision%29))
  (CallFunction|PlayerMovement (stale Input|AxisEvents|InputAxisleft-right AxisValue) AxisValue))

(event Input|AxisEvents|InputAxisleft-right
  (params (AxisValue :type Float%20%28single-precision%29))
  (CallFunction|PlayerMovement AxisValue (stale Input|AxisEvents|InputAxisfowards-backwards AxisValue)))

(fn ConstructionScript)

(fn TurnCameraon
  (CameraFades|StartCameraFade (Game|GetPlayerCameraManager 0) 1.0 0.0 2.0 "(R=0.000000,G=0.000000,B=0.000000,A=1.000000)" false false))

(fn RestartCurrentLevel
  (bind _returnvalue (Game|GetCurrentLevelName true))
  (Game|OpenLevel(byName) (Utilities|String|StringToName _returnvalue)))

(fn TurnCameraOff
  (bind _returnvalue (Math|Float|MakeLiteralFloat 2.0))
  (CameraFades|StartCameraFade (Game|GetPlayerCameraManager 0) 0.0 1.0 _returnvalue "(R=0.510417,G=0.009556,B=0.000000,A=1.000000)" false false)
  (return _returnvalue))

(fn PlayerMovement
  (params (A :type Float%20%28single-precision%29) (A2 :type Float%20%28single-precision%29))
  (bind _ballhorsepower (Variables|Default|GetBallHorsepower))
  (Class|PrimitiveComponent|AddTorqueinRadians (Variables|Default|GetBall) (Math|Vector|MakeVector (* A _ballhorsepower) (* A2 _ballhorsepower) 0.0) "None" true))

(fn AdjustCamera
  (params (Target%20Arm%20Length :type Float%20%28single-precision%29) (ArmRotation :type Rotator) (CameraRotation :type Rotator))
  (bind _springarm (Variables|Default|GetSpringArm))
  (Variables|/Script/Engine.SpringArmComponent|SetTargetArmLength _springarm Target%20Arm%20Length)
  (Transformation|SetRelativeRotation _springarm ArmRotation false false)
  (Transformation|SetRelativeRotation (Variables|Default|GetCamera) CameraRotation false false))